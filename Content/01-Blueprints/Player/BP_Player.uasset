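; BP_Player is a player Blueprint that sets up mouse cursor input and runs a periodic raycast from the cursor.
; BeginPlay shows the cursor, sets Game and UI input mode, and starts a looping 0.1-second timer calling MouseRaycast.
; MouseRaycast multi-traces on Visibility from the deprojected mouse location, deriving the end from that location rather than the mouse direction.
; The hits are unused, and each call prints a placeholder "Hello".
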(event `self.ReceiveBeginPlay`
  (bind _returnvalue (`GameplayStatics.GetPlayerController` 0))
  (set `PlayerController.bShowMouseCursor` true _returnvalue)
  (`WidgetBlueprintLibrary.SetInputMode_GameAndUIEx` _returnvalue null "LockOnCapture" false)
  (`KismetSystemLibrary.K2_SetTimer` null "MouseRaycast" 0.1 true true))

(fn `MouseRaycast`
  (bind _worldlocation (`PlayerController.DeprojectMousePositionToWorld` (`GameplayStatics.GetPlayerController` 0)))
  (`KismetSystemLibrary.LineTraceMulti` _worldlocation (+ (* _worldlocation (0.0 0.0 -1.0)) 500) "TraceTypeQuery1")
  (`KismetSystemLibrary.PrintString` "Hello"))

(fn `UserConstructionScript`)